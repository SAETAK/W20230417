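; BP_P39_Pawn is a player-controlled P-39 aircraft pawn that constantly flies forward along its local X axis.
; Pitch and Roll axis inputs rotate it locally, clamped and scaled by delta time and rotate speed.
; Tick also spins left and right propellers through RotatePropeller, but a three-second Delay precedes those calls, so they step only about once every three seconds rather than each frame.
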(event `self.ReceiveTick`
  (params (DeltaSeconds :type "Float (single-precision)"))
  ;[1 1 1] 앞으로 이동
  (`self.K2_AddActorLocalOffset` (`KismetMathLibrary.MakeVector` (* (`GameplayStatics.GetWorldDeltaSeconds`) (`self.MoveSpeed`))))
  (`KismetSystemLibrary.Delay` 3.0)
  ;[1 1 1] 왼쪽 프로펠러 회전
  (`self.RotatePropeller` (`self.Left`))
  ;[1 1 1] 오른쪽 프로펠러 회전
  (`self.RotatePropeller` (`self.Right`)))

(event `InputAxis|Pitch`
  (params (AxisValue :type "Float (single-precision)"))
  ;[1 1 1] Pitch 회전
  (`self.K2_AddActorLocalRotation` (`KismetMathLibrary.MakeRotator` 0.0 (* (`KismetMathLibrary.FClamp` AxisValue -1.0) (`GameplayStatics.GetWorldDeltaSeconds`) (`self.PlayerRotateSpeed`)))))

(event `InputAxis|Roll`
  (params (AxisValue :type "Float (single-precision)"))
  ;[1 1 1] Roll 회전
  (`self.K2_AddActorLocalRotation` (`KismetMathLibrary.MakeRotator` (* (`KismetMathLibrary.FClamp` AxisValue -1.0) (`GameplayStatics.GetWorldDeltaSeconds`) (`self.PlayerRotateSpeed`)))))

(fn `RotatePropeller`
  (params (Where :type "SceneComponent Object Reference"))
  (`SceneComponent.K2_AddRelativeRotation` Where (`KismetMathLibrary.MakeRotator` (* (`GameplayStatics.GetWorldDeltaSeconds`) (`self.PropellerRotateSpeed`))) false false))

(fn `UserConstructionScript`)